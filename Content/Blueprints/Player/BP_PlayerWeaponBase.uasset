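; Base player weapon Blueprint that displays the weapon as a Paper2D flipbook sprite with movement bob.
; A SceneCaptureComponent2D captures only the flipbook, and BeginPlay stores its relative location as the rest position.
; InitializeWeapon clears the flipbook and hides it in game.
; WeaponBob loops a sequence player while moving, otherwise stops it and interpolates the sprite back toward rest.
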(event `self.ReceiveBeginPlay`
  (`SceneCaptureComponent.ShowOnlyComponent` (`self.SceneCaptureComponent2D`) (`self.PaperFlipbook`))
  (set `self.WeaponPosition` (`SceneComponent.RelativeLocation` (`self.PaperFlipbook`))))

(event `/Game/Blueprints/Interfaces/IPlayerWeapon.InitializeWeapon`
  (bind _paperflipbook (`self.PaperFlipbook`))
  (`PaperFlipbookComponent.SetFlipbook` _paperflipbook null)
  (`SceneComponent.SetHiddenInGame` _paperflipbook true false))

(event `WeaponBob`
  (params (IsMoving :type Boolean) (DeltaTime :type "Float (double-precision)"))
  (bind _paperflipbook (`self.PaperFlipbook`))
  (bind _sequenceplayer (`ActorSequenceComponent.SequencePlayer` (`self.Weapon Bob`)))
  (if IsMoving
    (`MovieSceneSequencePlayer.PlayLooping` _sequenceplayer -1)
    (else
      (`MovieSceneSequencePlayer.Stop` _sequenceplayer)
      (`SceneComponent.K2_SetRelativeLocation` _paperflipbook (`KismetMathLibrary.VInterpTo` (`SceneComponent.RelativeLocation` _paperflipbook) (`self.WeaponPosition`) DeltaTime 5.0) false false))))

(fn `UserConstructionScript`)