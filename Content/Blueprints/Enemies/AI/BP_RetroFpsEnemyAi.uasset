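; Enemy AI for a retro FPS that turns perception of Player-tagged actors into Blackboard state.
; On a successful sense, it cancels the lost-sight timer, sets CanSeeTarget and stores the player as TargetActor.
; When sensing fails, it clears CanSeeTarget at once but keeps TargetActor until a short timer expires, giving the enemy a brief memory of the player.
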(event `self.AIPerception.OnTargetPerceptionUpdated`
  (params (Actor :type "Actor Object Reference") (Stimulus :type "AIStimulus Structure"))
  (bind _output_get (set `self.PerceivedActor` Actor))
  (if (`self.ActorHasTag` _output_get "Player")
    (if Stimulus_bSuccessfullySensed
      (`KismetSystemLibrary.K2_ClearAndInvalidateTimerHandle` (`self.Lost sight timer`))
      (`self.UpdateSightKey` true)
      (`self.UpdateTargetKey` (`self.PerceivedActor`))
      (else
        (bind _returnvalue (`KismetSystemLibrary.K2_SetTimerDelegate` (delegate `Lost sight`) 5.0))
        (set `self.Lost sight timer` _returnvalue)
        (`self.UpdateSightKey` false)))))

(event `Lost sight`
  (`self.UpdateTargetKey` null))

(fn `UpdateSightKey`
  (params (CanSeePlayer :type Boolean))
  (`BlackboardComponent.SetValueAsBool` (`AIBlueprintHelperLibrary.GetBlackboard` null) "CanSeeTarget" CanSeePlayer))

(fn `UpdateTargetKey`
  (params (`Target actor` :type "Actor Object Reference"))
  (`BlackboardComponent.SetValueAsObject` (`AIBlueprintHelperLibrary.GetBlackboard` null) "TargetActor" `Target actor`))

(fn `UserConstructionScript`)