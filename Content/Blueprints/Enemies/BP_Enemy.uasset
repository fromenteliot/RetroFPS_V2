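; Enemy actor drawn as a billboarded Paper2D flipbook with directional sprites, with HP-based damage that destroys it at zero.
; Each tick it yaws the sprite toward the camera, then, unless dead or paused, measures the player's angle against its forward vector.
; Angle and side select front, left or right flipbooks; there is no back view.
; CheckIfWalking sets IsWalking true on both branches, so idle flipbooks are never selected.
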(event `self.ReceiveTick`
  (params (DeltaSeconds :type "Float (single-precision)"))
  (`self.SpriteFacePlayer`
    (:`Out`
      (if (not (or (`self.IsDead`) (`self.Pause Angle Calculations`)))
        (`self.GetEnemyAngle`
          (:`Out`
            (`self.CheckIfWalking`
              (:`Out`
                (`self.CalculateFlipbook`)))))))))

(event `/Game/Blueprints/Interfaces/IDamageable.Kill`
  (`self.K2_DestroyActor`))

(fn `Damage`
  (params (Damage :type "Float (double-precision)"))
  (returns (Killed :type Boolean))
  (bind _output_get (set `self.HP` (- (`self.HP`) Damage)))
  (if (<= _output_get 0.0)
    (`self.Kill`)
    (return true)
    (else
      (return false))))

(fn `SetFlipbook`
  (params (Walking :type "PaperFlipbook Object Reference") (Idle :type "PaperFlipbook Object Reference"))
  (bind _paperflipbook (`self.PaperFlipbook`))
  (if (`self.IsWalking`)
    (`PaperFlipbookComponent.SetFlipbook` _paperflipbook Walking)
    (else
      (`PaperFlipbookComponent.SetFlipbook` _paperflipbook Idle))))

(fn `UserConstructionScript`)