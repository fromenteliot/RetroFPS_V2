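; Player punch gameplay ability for the retro FPS player, dealing melee damage and rewarding kills with health.
; FireWeapon lazily caches the owning player and the BP_Punch actor in its weapon child-actor slot, then plays the punch animation.
; It sends Damage through the IDamageable interface to every actor overlapping the player, with no trace or aim check.
; Each DamageMessage that returns true heals the player by HealOnKill.
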(event `self.FireWeapon`
  (bind _playerpunchweaponcomponent (`self.PlayerPunchWeaponComponent`))
  (`self.GetPlayer`)
  (`self.GetWeapon`)
  (`/Engine/EditorBlueprintResources/StandardMacros.IsValid` _playerpunchweaponcomponent
    (:`Is Valid`
      (`/Game/Blueprints/Weapons/BP_Punch.PunchAnim` _playerpunchweaponcomponent)
      (for _array_element (`Actor.GetOverlappingActors` (`self.Player`) null)
        (if (`KismetSystemLibrary.DoesImplementInterface` _array_element "/Game/Blueprints/Interfaces/IDamageable.IDamageable_C")
          (bind _killed (message `/Game/Blueprints/Interfaces/IDamageable.Damage` _array_element (`self.Damage`)))
          (if _killed
            (`/Game/Blueprints/Player/BP_RetroFpsPlayer.Heal` (`self.Player`) (`self.Heal On Kill`))))))))

(fn `GetPlayer`
  (bind _returnvalue_owneractor (break `GameplayAbilityActorInfo` (`self.GetActorInfo`)))
  (`/Engine/EditorBlueprintResources/StandardMacros.IsValid` (`self.Player`)
    (:`Is Valid`
      _)
    (:`Is Not Valid`
      (bind _asbp_retro_fps_player (cast `/Game/Blueprints/Player/BP_RetroFpsPlayer` _returnvalue_owneractor))
      (set `self.Player` _asbp_retro_fps_player)))
  (return))

(fn `GetWeapon`
  (`/Engine/EditorBlueprintResources/StandardMacros.IsValid` (`self.PlayerPunchWeaponComponent`)
    (:`Is Valid`
      _)
    (:`Is Not Valid`
      (bind _asbp_punch (cast `/Game/Blueprints/Weapons/BP_Punch` (`ChildActorComponent.ChildActor` (`/Game/Blueprints/Player/BP_RetroFpsPlayer.Weapon` (`self.Player`)))))
      (set `self.PlayerPunchWeaponComponent` _asbp_punch)))
  (return))