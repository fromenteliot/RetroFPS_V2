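; Gameplay ability for the player pistol's alternate fire: a hitscan shot that ricochets off surfaces.
; FireWeapon traces from the camera, reflecting the direction about each impact normal until it misses, reaches the rebound limit or hits an IDamageable actor.
; Damage to that actor grows linearly with the bounce count.
; The pistol class is added to the player's WeaponCD after the shot and removed after a delay, blocking refire during cooldown.
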(event `self.FireWeapon`
  (bind _playerpistolweaponcomponent (`self.PlayerPistolWeaponComponent`))
  (bind _damage (`self.Damage`))
  (bind _returnvalue (`GameplayStatics.GetObjectClass` (`self.PlayerPistolWeaponComponent`)))
  (bind _camera (`/Game/Blueprints/Player/BP_RetroFpsPlayer.Camera` (`self.Player`)))
  (bind _weapon_cd (`/Game/Blueprints/Player/BP_RetroFpsPlayer.Weapon CD` (`self.Player`)))
  (`self.GetPlayer`)
  (`self.GetWeapon`)
  (`/Engine/EditorBlueprintResources/StandardMacros.IsValid` _playerpistolweaponcomponent
    (:`Is Valid`
      (if (not (`BlueprintSetLibrary.Set_Contains` (`/Game/Blueprints/Player/BP_RetroFpsPlayer.Weapon CD` (`self.Player`)) (`GameplayStatics.GetObjectClass` _playerpistolweaponcomponent)))
        (`/Game/Blueprints/Weapons/BP_Pistol.ShootPistol` _playerpistolweaponcomponent)
        (set `self.Start` (`SceneComponent.K2_GetComponentLocation` _camera))
        (set `self.Ignore` (`self.Player`))
        (set `self.Direction` (`SceneComponent.K2_GetComponentRotation` _camera))
        (for _index (range (+ (`self.MaxRebounds`) 1))
          (bind (_actor _impactpoint _bounceddirection _hit) (`self.Get Line Trace` (`self.Start`) (`self.Direction`) (`self.Ignore`)))
          (if _hit
            (if (`KismetSystemLibrary.DoesImplementInterface` _actor "/Game/Blueprints/Interfaces/IDamageable.IDamageable_C")
              ;[1 1 1] If hit si damageable, apply damage
              (message `/Game/Blueprints/Interfaces/IDamageable.Damage` _actor (+ _damage (* _damage _index)))
              (break)
              (else
                (set `self.Start` _impactpoint)
                (set `self.Direction` _bounceddirection)
                (set `self.Ignore` _actor)))
            (else
              (break))))
        (`BlueprintSetLibrary.Set_Add` _weapon_cd _returnvalue)
        (`KismetSystemLibrary.Delay` (`self.Cooldown`))
        (`BlueprintSetLibrary.Set_Remove` _weapon_cd _returnvalue)))))

(fn `Get Line Trace`
  (params (Start :type "Vector Structure") (Forward :type "Rotator Structure") (Ignore :type "Actor Object Reference"))
  (returns (Actor :type "Actor Object Reference") (ImpactPoint :type "Vector Structure") (BouncedDirection :type "Rotator Structure") (Hit :type Boolean))
  (bind _returnvalue (+ Start (* (`KismetMathLibrary.GetForwardVector` Forward) (`self.WeaponRange`))))
  (bind _returnvalue_2 (`KismetMathLibrary.Normal` (- _returnvalue Start)))
  (bind _outhit (`KismetSystemLibrary.LineTraceSingle` Start _returnvalue "TraceTypeQuery3" false (`|MakeArray` Ignore)))
  (bind (_bblockinghit _binitialoverlap _time _distance _location _impactpoint _normal _impactnormal _physmat _hitactor) (`GameplayStatics.BreakHitResult` _outhit))
  (return _hitactor _impactpoint (`KismetMathLibrary.Conv_VectorToRotator` (- _returnvalue_2 (* (* (`KismetMathLibrary.Dot_VectorVector` _returnvalue_2 _impactnormal) 2.0) _impactnormal))) _bblockinghit))

(fn `GetPlayer`
  (bind _returnvalue_owneractor (break `GameplayAbilityActorInfo` (`self.GetActorInfo`)))
  (`/Engine/EditorBlueprintResources/StandardMacros.IsValid` (`self.Player`)
    (:`Is Valid`
      _)
    (:`Is Not Valid`
      (bind _asbp_retro_fps_player (cast `/Game/Blueprints/Player/BP_RetroFpsPlayer` _returnvalue_owneractor))
      (set `self.Player` _asbp_retro_fps_player)))
  (return))

(fn `GetWeapon`
  (`/Engine/EditorBlueprintResources/StandardMacros.IsValid` (`self.PlayerPistolWeaponComponent`)
    (:`Is Valid`
      _)
    (:`Is Not Valid`
      (bind _asbp_pistol (cast `/Game/Blueprints/Weapons/BP_Pistol` (`ChildActorComponent.ChildActor` (`/Game/Blueprints/Player/BP_RetroFpsPlayer.Weapon` (`self.Player`)))))
      (set `self.PlayerPistolWeaponComponent` _asbp_pistol)))
  (return))