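; Shotgun alt-fire gameplay ability for the retro FPS player that pumps the weapon instead of shooting.
; FireWeapon raises the shotgun's PumpLevel by one, as long as it stays within MaxPumps.
; Helper functions lazily cache the player from the ability's owner actor and the BP_Shotgun from the player's Weapon child actor.
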(event `self.FireWeapon`
  (bind _playershotgunweaponcomponent (`self.PlayerShotgunWeaponComponent`))
  (bind _returnvalue (+ 1 (`/Game/Blueprints/Weapons/BP_Shotgun.PumpLevel` _playershotgunweaponcomponent)))
  (`self.GetPlayer`)
  (`self.GetWeapon`)
  (`/Engine/EditorBlueprintResources/StandardMacros.IsValid` _playershotgunweaponcomponent
    (:`Is Valid`
      (if (>= (`/Game/Blueprints/Weapons/BP_Shotgun.MaxPumps` _playershotgunweaponcomponent) _returnvalue)
        (set `/Game/Blueprints/Weapons/BP_Shotgun.PumpLevel` _returnvalue _playershotgunweaponcomponent)))))

(fn `GetPlayer`
  (bind _returnvalue_owneractor (break `GameplayAbilityActorInfo` (`self.GetActorInfo`)))
  (`/Engine/EditorBlueprintResources/StandardMacros.IsValid` (`self.Player`)
    (:`Is Valid`
      _)
    (:`Is Not Valid`
      (bind _asbp_retro_fps_player (cast `/Game/Blueprints/Player/BP_RetroFpsPlayer` _returnvalue_owneractor))
      (set `self.Player` _asbp_retro_fps_player)))
  (return))

(fn `GetWeapon`
  (`/Engine/EditorBlueprintResources/StandardMacros.IsValid` (`self.PlayerShotgunWeaponComponent`)
    (:`Is Valid`
      _)
    (:`Is Not Valid`
      (bind _asbp_shotgun (cast `/Game/Blueprints/Weapons/BP_Shotgun` (`ChildActorComponent.ChildActor` (`/Game/Blueprints/Player/BP_RetroFpsPlayer.Weapon` (`self.Player`)))))
      (set `self.PlayerShotgunWeaponComponent` _asbp_shotgun)))
  (return))