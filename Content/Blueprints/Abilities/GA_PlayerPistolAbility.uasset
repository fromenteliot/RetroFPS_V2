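; Player pistol gameplay ability that fires the pistol and applies an effect to the character under the player's aim.
; FireWeapon lazily caches the owning BP_Player and its BP_Pistol child actor, then calls ShootPistol on the pistol.
; A Visibility line trace along the camera's forward vector out to WeaponRange finds the target.
; ApplyEffect runs only when the hit actor is a RetroFPSCharacter.
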(event `self.FireWeapon`
  (bind _playerpistolweaponcomponent (`self.PlayerPistolWeaponComponent`))
  (`self.GetPlayer`)
  (`self.GetWeapon`)
  (`/Engine/EditorBlueprintResources/StandardMacros.IsValid` _playerpistolweaponcomponent
    (:`Is Valid`
      (`/Game/Blueprints/Weapons/BP_Pistol.ShootPistol` _playerpistolweaponcomponent)
      (bind _actor (`self.Get Line Trace`))
      (bind _asretro_fpscharacter (cast `RetroFPSCharacter` _actor))
      (`self.Apply Effect` (`self.Player`) _asretro_fpscharacter))))

(fn `Get Line Trace`
  (returns (Actor :type "Actor Object Reference"))
  (bind _camera (`/Game/Blueprints/Player/BP_Player.Camera` (`self.Player`)))
  (bind _returnvalue (`SceneComponent.K2_GetComponentLocation` _camera))
  (bind _outhit (`KismetSystemLibrary.LineTraceSingle` _returnvalue (+ _returnvalue (* (`KismetMathLibrary.GetForwardVector` (`SceneComponent.K2_GetComponentRotation` _camera)) (`self.WeaponRange`))) "TraceTypeQuery1"))
  (bind (_bblockinghit _binitialoverlap _time _distance _location _impactpoint _normal _impactnormal _physmat _hitactor) (`GameplayStatics.BreakHitResult` _outhit))
  (`/Engine/EditorBlueprintResources/StandardMacros.IsValid` _hitactor
    (:`Is Valid`
      (return _hitactor))))

(fn `GetPlayer`
  (bind _returnvalue_owneractor (break `GameplayAbilityActorInfo` (`self.GetActorInfo`)))
  (`/Engine/EditorBlueprintResources/StandardMacros.IsValid` (`self.Player`)
    (:`Is Valid`
      _)
    (:`Is Not Valid`
      (bind _asbp_player (cast `/Game/Blueprints/Player/BP_Player` _returnvalue_owneractor))
      (set `self.Player` _asbp_player)))
  (return))

(fn `GetWeapon`
  (`/Engine/EditorBlueprintResources/StandardMacros.IsValid` (`self.PlayerPistolWeaponComponent`)
    (:`Is Valid`
      _)
    (:`Is Not Valid`
      (bind _asbp_pistol (cast `/Game/Blueprints/Weapons/BP_Pistol` (`ChildActorComponent.ChildActor` (`/Game/Blueprints/Player/BP_Player.Weapon` (`self.Player`)))))
      (set `self.PlayerPistolWeaponComponent` _asbp_pistol)))
  (return))