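; GA_BFGAbilityAlt is an alternate BFG gameplay ability that spawns a Mine actor from the player's camera.
; FireWeapon lazily caches the owning BP_RetroFpsPlayer and its weapon child actor, which must cast to BP_Mine.
; With a valid weapon, it spawns the mine at the camera's position and rotation once the cooldown since LastUse has elapsed.
; LastUse is read but never updated in this graph.
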(event `self.FireWeapon`
  (bind _camera (`/Game/Blueprints/Player/BP_RetroFpsPlayer.Camera` (`self.Player`)))
  (`self.GetPlayer`)
  (`self.GetWeapon`)
  (`/Engine/EditorBlueprintResources/StandardMacros.IsValid` (`self.PleayerMineComponent`)
    (:`Is Valid`
      (if (> (`KismetMathLibrary.Now`) (+ (`self.LastUse`) (`KismetMathLibrary.FromSeconds` (`self.Cooldown`))))
        (`|SpawnActorFromClass` (`self.Mine`) (`KismetMathLibrary.MakeTransform` (`SceneComponent.K2_GetComponentLocation` _camera) (`SceneComponent.K2_GetComponentRotation` _camera)) "AlwaysSpawn" "OverrideRootScale" null null)))))

(fn `GetPlayer`
  (bind _returnvalue_owneractor (break `GameplayAbilityActorInfo` (`self.GetActorInfo`)))
  (`/Engine/EditorBlueprintResources/StandardMacros.IsValid` (`self.Player`)
    (:`Is Valid`
      _)
    (:`Is Not Valid`
      (bind _asbp_retro_fps_player (cast `/Game/Blueprints/Player/BP_RetroFpsPlayer` _returnvalue_owneractor))
      (set `self.Player` _asbp_retro_fps_player)))
  (return))

(fn `GetWeapon`
  (`/Engine/EditorBlueprintResources/StandardMacros.IsValid` (`self.PleayerMineComponent`)
    (:`Is Valid`
      _)
    (:`Is Not Valid`
      (bind _asbp_mine (cast `/Game/Blueprints/Weapons/BP_Mine` (`ChildActorComponent.ChildActor` (`/Game/Blueprints/Player/BP_RetroFpsPlayer.Weapon` (`self.Player`)))))
      (set `self.PleayerMineComponent` _asbp_mine)))
  (return))