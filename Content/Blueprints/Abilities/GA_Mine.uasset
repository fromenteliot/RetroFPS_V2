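; Destructible mine actor that deals area damage when its health runs out.
; Damage subtracts from HP, calls Kill at zero or below, and returns whether the mine died.
; Kill runs a multi-sphere trace at the mine's location, sends DamageMessage to hit actors implementing IDamageable, then destroys itself.
; There is no proximity or timer trigger; overlap and tick events are unused.
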(event `/Game/Blueprints/Interfaces/IDamageable.Kill`
  (bind _returnvalue (`SceneComponent.K2_GetComponentLocation` (`self.Mine`)))
  (bind _outhits (`KismetSystemLibrary.SphereTraceMulti` _returnvalue _returnvalue (`self.Radius`) "TraceTypeQuery3"))
  (for _array_element _outhits
    (bind (_bblockinghit _binitialoverlap _time _distance _location _impactpoint _normal _impactnormal _physmat _hitactor) (`GameplayStatics.BreakHitResult` _array_element))
    (if (`KismetSystemLibrary.DoesImplementInterface` _hitactor "/Game/Blueprints/Interfaces/IDamageable.IDamageable_C")
      (message `/Game/Blueprints/Interfaces/IDamageable.Damage` _hitactor (`self.Dmg`))))
  (`self.K2_DestroyActor`))

(fn `Damage`
  (params (Damage :type "Float (double-precision)"))
  (returns (Killed :type Boolean))
  (bind _output_get (set `self.HP` (- (`self.HP`) Damage)))
  (if (<= _output_get 0.0)
    (`self.Kill`)
    (return true)
    (else
      (return false))))

(fn `UserConstructionScript`)