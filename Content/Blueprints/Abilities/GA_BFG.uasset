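; BFG ability actor that acts as either a moving damage projectile (main fire) or a destructible mine (alt fire), selected by IsPhys.
; In projectile mode, Tick advances it and sphere-traces damage to IDamageable actors each frame until its duration expires.
; Otherwise, incoming damage drains HP until Kill triggers a radial trace.
; The mine destroys itself before messaging hit actors, preventing infinite loops between chained mines.
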(event `/Game/Blueprints/Interfaces/IDamageable.Kill`
  (bind _returnvalue (`SceneComponent.K2_GetComponentLocation` (`self.Mine`)))
  ;[1 1 1] On Killed (Alt Fire)
  (`self.ApplyDamage` _returnvalue _returnvalue (`self.Radius`) true))

(event `self.ReceiveTick`
  (params (DeltaSeconds :type "Float (single-precision)"))
  (bind _returnvalue (`SceneComponent.K2_GetComponentLocation` (`self.Mine`)))
  ;[1 1 1] Damage Loop (Main Fire)
  (if (`self.IsPhys`)
    (bind _output_get (set `self.Duration` (- (`self.Duration`) DeltaSeconds)))
    (if (<= _output_get 0.0)
      (`self.K2_DestroyActor`)
      (else
        (`SceneComponent.K2_AddWorldOffset` (`self.Mine`) (* (`self.Speed`) (`SceneComponent.GetForwardVector` (`self.Mine`))) false false)
        (`self.ApplyDamage` _returnvalue _returnvalue (`self.MovingRadius`) false (`self.Dmp Per Tick`))))))

(fn `ApplyDamage`
  (params (Start :type "Vector Structure") (End :type "Vector Structure") (Radius :type "Float (single-precision)") (IsMine :type Boolean) (Damage :type "Float (double-precision)"))
  (bind _outhits (`KismetSystemLibrary.SphereTraceMulti` Start End Radius "TraceTypeQuery3"))
  (if IsMine
    (`self.K2_DestroyActor`) ; If is in mine mode, destroy before loop to avoid multiple mines causing an infinite loop
  )
  (for _array_element _outhits
    (bind (_bblockinghit _binitialoverlap _time _distance _location _impactpoint _normal _impactnormal _physmat _hitactor) (`GameplayStatics.BreakHitResult` _array_element))
    (if (`KismetSystemLibrary.DoesImplementInterface` _hitactor "/Game/Blueprints/Interfaces/IDamageable.IDamageable_C")
      (message `/Game/Blueprints/Interfaces/IDamageable.Damage` _hitactor Damage))))

(fn `Damage`
  (params (Damage :type "Float (double-precision)"))
  (returns (Killed :type Boolean))
  (if (`self.IsPhys`)
    (return false)
    (else
      (bind _output_get (set `self.HP` (- (`self.HP`) Damage)))
      (if (<= _output_get 0.0)
        (`self.Kill`)
        (return true)
        (else
          (return false))))))

(fn `UserConstructionScript`)