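; Player shotgun gameplay ability that fires multiple hitscan pellets from the retro FPS player's camera.
; FireWeapon caches the player and shotgun child actor, then runs a debug-drawn line trace per pellet.
; Trace endpoints get random square-root-scaled polar offsets on world X and Z for spread.
; Hit actors implementing IDamageable receive DamageMessage, and the loop stops at the first one returning true.
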(event `self.FireWeapon`
  (`self.GetPlayer`)
  (`self.GetWeapon`)
  (`/Engine/EditorBlueprintResources/StandardMacros.IsValid` (`self.PlayerShotgunWeaponComponent`)
    (:`Is Valid`
      (for _ (range (+ (`self.Pellets`) 1))
        (bind _actor (`self.Get Line Trace`))
        (if (`KismetSystemLibrary.DoesImplementInterface` _actor "/Game/Blueprints/Interfaces/IDamageable.IDamageable_C")
          (bind _killed (message `/Game/Blueprints/Interfaces/IDamageable.Damage` _actor (`self.Damage`)))
          (if _killed
            (break)))))))

(fn `Get Line Trace`
  (returns (Actor :type "Actor Object Reference"))
  (bind _coneradius (`self.ConeRadius`))
  (bind _camera (`/Game/Blueprints/Player/BP_RetroFpsPlayer.Camera` (`self.Player`)))
  (bind _returnvalue (`SceneComponent.K2_GetComponentLocation` _camera))
  (bind _returnvalue_2 (`KismetMathLibrary.RandomFloatInRange` 0.0 (* 2.0 (`KismetMathLibrary.GetPI`))))
  (bind _returnvalue_3 (`KismetMathLibrary.Sqrt` (* (`KismetMathLibrary.RandomFloatInRange` 0.0 _coneradius) _coneradius)))
  (bind _outhit (`KismetSystemLibrary.LineTraceSingle` :`Start` _returnvalue :`End` (+ (+ _returnvalue (* (`KismetMathLibrary.GetForwardVector` (`SceneComponent.K2_GetComponentRotation` _camera)) (`self.WeaponRange`))) (`KismetMathLibrary.MakeVector` (* (`KismetMathLibrary.Cos` _returnvalue_2) _returnvalue_3) 0.0 (* (`KismetMathLibrary.Sin` _returnvalue_2) _returnvalue_3))) :`TraceChannel` "TraceTypeQuery3" :`DrawDebugType` "ForDuration"))
  (bind (_bblockinghit _binitialoverlap _time _distance _location _impactpoint _normal _impactnormal _physmat _hitactor) (`GameplayStatics.BreakHitResult` _outhit))
  (`/Engine/EditorBlueprintResources/StandardMacros.IsValid` _hitactor
    (:`Is Valid`
      (return _hitactor))))

(fn `GetPlayer`
  (bind _returnvalue_owneractor (break `GameplayAbilityActorInfo` (`self.GetActorInfo`)))
  (`/Engine/EditorBlueprintResources/StandardMacros.IsValid` (`self.Player`)
    (:`Is Valid`
      _)
    (:`Is Not Valid`
      (bind _asbp_retro_fps_player (cast `/Game/Blueprints/Player/BP_RetroFpsPlayer` _returnvalue_owneractor))
      (set `self.Player` _asbp_retro_fps_player)))
  (return))

(fn `GetWeapon`
  (`/Engine/EditorBlueprintResources/StandardMacros.IsValid` (`self.PlayerShotgunWeaponComponent`)
    (:`Is Valid`
      _)
    (:`Is Not Valid`
      (bind _asbp_shotgun (cast `/Game/Blueprints/Weapons/BP_Shotgun` (`ChildActorComponent.ChildActor` (`/Game/Blueprints/Player/BP_RetroFpsPlayer.Weapon` (`self.Player`)))))
      (set `self.PlayerShotgunWeaponComponent` _asbp_shotgun)))
  (return))