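; Base weapon gameplay ability for a retro FPS, with FireWeapon and Reset left as empty hooks.
; Activation commits, listens for the weapon event tag, fires, then ends after the remaining cooldown, pacing fire rate.
; ApplyEffect sends hit RetroFPSCharacter targets to the attacker's instigator as a gameplay event, whose listener applies the weapon effect.
; Ending cleans up both async tasks and calls Reset, behind nested validity checks.
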(event `FireWeapon`)

(event `self.K2_ActivateAbility`
  (`self.K2_CommitAbility`)
  (`self.WaitForEvent`)
  (`self.FireWeapon`)
  (bind _asynctaskproxy (`GameplayTask_WaitDelay.TaskWaitDelay` null (`self.GetCooldownTimeRemaining`))
    (:`then`
      (set `self.FireRateDelayTask` _asynctaskproxy))
    (:`OnFinish`
      (`self.K2_EndAbility`))))

(event `WaitForEvent`
  ;[1 1 1] Wait for gameplay tag
  (bind (_asynctaskproxy _payload) (`AbilityTask_WaitGameplayEvent.WaitGameplayEvent` (`self.Weapon Event  Tag`) null)
    (:`then`
      (set `self.Gameplay Event Wait Task` _asynctaskproxy))
    (:`EventReceived`
      (`self.BP_ApplyGameplayEffectToTarget` (`.TargetData` (break `GameplayEventData` _payload)) (`self.WeaponEffect`)))))

(event `self.K2_OnEndAbility`
  (params (bWasCancelled :type Boolean))
  (bind _gameplay_event_wait_task (`self.Gameplay Event Wait Task`))
  (bind _fireratedelaytask (`self.FireRateDelayTask`))
  ;[1 1 1] End Cleanup
  (`/Engine/EditorBlueprintResources/StandardMacros.IsValid` _gameplay_event_wait_task
    (:`Is Valid`
      (`GameplayTask.EndTask` _gameplay_event_wait_task)
      (`/Engine/EditorBlueprintResources/StandardMacros.IsValid` _fireratedelaytask
        (:`Is Valid`
          (`GameplayTask.EndTask` _fireratedelaytask)
          (`self.Reset`))))))

(fn `Apply Effect`
  (params (AttackingActor :type "Actor Object Reference") (TargetActor :type "Actor Object Reference"))
  ;[1 1 1] Equip Weapon
  (bind _asretro_fpscharacter (cast `RetroFPSCharacter` TargetActor))
  (`AbilitySystemBlueprintLibrary.SendGameplayEventToActor` (`Actor.Instigator` AttackingActor) (`self.Weapon Event  Tag`) (make `GameplayEventData` (struct) null _asretro_fpscharacter null null (struct) (struct) (struct) 0.0 (`AbilitySystemBlueprintLibrary.AbilityTargetDataFromActor` _asretro_fpscharacter))))

(fn `Reset`)