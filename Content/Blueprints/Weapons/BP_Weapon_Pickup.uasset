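; BP_Weapon_Pickup is a world pickup that gives its Weapon to the player on touch.
; When a BP_Player overlaps it, the pickup calls EquipWeapon on that player and destroys itself.
; Every tick it billboards its Paper flipbook toward player 0's camera on yaw only, offset by 90 degrees so the sprite stays upright and faces the view.
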(event `self.ReceiveActorBeginOverlap`
  (params (OtherActor :type "Actor Object Reference"))
  (bind _asbp_player (cast `/Game/Blueprints/Player/BP_Player` OtherActor))
  (`/Game/Blueprints/Player/BP_Player.EquipWeapon` _asbp_player (`self.Weapon`))
  (`self.K2_DestroyActor`))

(event `self.ReceiveTick`
  (params (DeltaSeconds :type "Float (single-precision)"))
  (bind _paperflipbookthatcrashesthegame (`self.PaperFlipbookThatCrashesTheGame`))
  (bind (_returnvalue_roll _returnvalue_pitch _returnvalue_yaw) (`KismetMathLibrary.BreakRotator` (`KismetMathLibrary.FindLookAtRotation` (`SceneComponent.K2_GetComponentLocation` _paperflipbookthatcrashesthegame) (`PlayerCameraManager.GetCameraLocation` (`GameplayStatics.GetPlayerCameraManager` 0)))))
  (`SceneComponent.K2_SetWorldRotation` _paperflipbookthatcrashesthegame (`KismetMathLibrary.MakeRotator` 0.0 0.0 (- _returnvalue_yaw 90.0)) false false))

(fn `UserConstructionScript`)