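; BP_Pistol is a hitscan pistol weapon drawn with Paper2D flipbooks, attached as a child actor of a camera owner.
; Firing plays the fire flipbook before returning to idle, briefly flashes a point light and runs HitScan.
; HitScan line-traces from the parent's camera to forward times Range, without adding the start location, and sends damage through IDamageable.
; Debug trace drawing and printed hit names remain active.
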(event `/Game/Blueprints/Interfaces/IPlayerWeapon.InitializeWeapon`
  ;[1 1 1] Equip weapon
  (`PaperFlipbookComponent.SetFlipbook` (`self.PaperFlipbook`) (`self.IdleFlipbook`))
  (`SceneComponent.SetHiddenInGame` (`self.PaperFlipbook`) false false))

(event `ShootPistol`
  (bind _paperflipbook (`self.PaperFlipbook`))
  ;[1 1 1] Fire animation
  (`self.Light Flash`)
  (`PaperFlipbookComponent.SetFlipbook` _paperflipbook (`self.FireFlipbook`))
  (`self.HitScan`)
  (`KismetSystemLibrary.Delay` (`PaperFlipbookComponent.GetFlipbookLength` _paperflipbook))
  (`PaperFlipbookComponent.SetFlipbook` (`self.PaperFlipbook`) (`self.IdleFlipbook`)))

(event `Light Flash`
  (bind _pointlight (`self.PointLight`))
  ;[1 1 1] Light flash
  (`SceneComponent.SetHiddenInGame` _pointlight false false)
  (`KismetSystemLibrary.Delay` 0.1)
  (`SceneComponent.SetHiddenInGame` _pointlight true false))

(fn `HitScan`
  (bind _returnvalue (`self.GetComponentByClass` (`self.GetParentActor`) "/Script/Engine.CameraComponent"))
  (bind (_outhit _returnvalue_2) (`KismetSystemLibrary.LineTraceSingle` :`Start` (`SceneComponent.K2_GetComponentLocation` _returnvalue) :`End` (* (`KismetMathLibrary.GetForwardVector` (`SceneComponent.K2_GetComponentRotation` _returnvalue)) (`self.Range`)) :`TraceChannel` "TraceTypeQuery3" :`DrawDebugType` "ForDuration"))
  (`KismetSystemLibrary.PrintText` "Shot")
  (bind (_bblockinghit _binitialoverlap _time _distance _location _impactpoint _normal _impactnormal _physmat _hitactor) (`GameplayStatics.BreakHitResult` _outhit))
  (`KismetSystemLibrary.PrintString` (`KismetSystemLibrary.GetDisplayName` _hitactor))
  (if _returnvalue_2
    (if (`KismetSystemLibrary.DoesImplementInterface` _hitactor "/Game/Blueprints/Interfaces/IDamageable.IDamageable_C")
      (message `/Game/Blueprints/Interfaces/IDamageable.Damage` _hitactor (`self.Damage`)))))

(fn `UserConstructionScript`
  (`parent.UserConstructionScript`))