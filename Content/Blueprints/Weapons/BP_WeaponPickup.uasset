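; BP_WeaponPickup is a weapon pickup actor for a retro FPS player.
; On overlap with BP_RetroFpsPlayer, it equips its ThisWeapon on that player and destroys itself.
; Every tick it billboards its Paper2D flipbook by yawing it toward the player camera with a 90-degree offset, keeping pitch and roll at zero.
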(event `self.ReceiveActorBeginOverlap`
  (params (OtherActor :type "Actor Object Reference"))
  (bind _asbp_retro_fps_player (cast `/Game/Blueprints/Player/BP_RetroFpsPlayer` OtherActor))
  (`/Game/Blueprints/Player/BP_RetroFpsPlayer.EquipWeapon` _asbp_retro_fps_player (`self.ThisWeapon`))
  (`self.K2_DestroyActor`))

(event `self.ReceiveTick`
  (params (DeltaSeconds :type "Float (single-precision)"))
  (bind _paperflipbook (`self.PaperFlipbook`))
  (bind (_returnvalue_roll _returnvalue_pitch _returnvalue_yaw) (`KismetMathLibrary.BreakRotator` (`KismetMathLibrary.FindLookAtRotation` (`SceneComponent.K2_GetComponentLocation` _paperflipbook) (`PlayerCameraManager.GetCameraLocation` (`GameplayStatics.GetPlayerCameraManager` 0)))))
  (`SceneComponent.K2_SetWorldRotation` _paperflipbook (`KismetMathLibrary.MakeRotator` 0.0 0.0 (- _returnvalue_yaw 90.0)) false false))

(fn `UserConstructionScript`)