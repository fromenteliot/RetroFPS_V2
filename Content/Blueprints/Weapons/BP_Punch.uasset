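; BP_Punch is a punch weapon Blueprint that displays its idle and attack animations through a Paper2D flipbook.
; InitializeWeapon sets the idle flipbook and makes the component visible when the weapon is equipped.
; PunchAnim switches to the fire flipbook, waits for its length with a Delay, then returns to idle.
; The file holds only this visual logic, with no hit or damage handling, and its construction script just calls the parent.
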(event `self.InitializeWeapon`
  ;[1 1 1] Equip weapon
  (`PaperFlipbookComponent.SetFlipbook` (`self.PaperFlipbook`) (`self.IdleFlipbook`))
  (`SceneComponent.SetHiddenInGame` (`self.PaperFlipbook`) false false))

(event `PunchAnim`
  (bind _paperflipbook (`self.PaperFlipbook`))
  ;[1 1 1] Fire animation
  (`PaperFlipbookComponent.SetFlipbook` _paperflipbook (`self.FireFlipbook`))
  (`KismetSystemLibrary.Delay` (`PaperFlipbookComponent.GetFlipbookLength` _paperflipbook))
  (`PaperFlipbookComponent.SetFlipbook` (`self.PaperFlipbook`) (`self.IdleFlipbook`)))

(fn `UserConstructionScript`
  (`parent.UserConstructionScript`))