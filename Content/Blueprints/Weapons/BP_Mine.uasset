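; BP_Mine is a weapon Blueprint that handles flipbook visuals and a light flash for equipping and firing.
; InitializeWeapon shows the idle flipbook, while ShootPistol plays the fire flipbook for its length and then returns to idle.
; Each shot also calls LightFlash, which briefly unhides a point light.
; Despite the Mine name, the fire event is named ShootPistol, and the graph contains no projectile, damage or explosion logic.
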(event `self.InitializeWeapon`
  ;[1 1 1] Equip weapon
  (`PaperFlipbookComponent.SetFlipbook` (`self.PaperFlipbook`) (`self.IdleFlipbook`))
  (`SceneComponent.SetHiddenInGame` (`self.PaperFlipbook`) false false))

(event `ShootPistol`
  (bind _paperflipbook (`self.PaperFlipbook`))
  ;[1 1 1] Fire animation
  (`self.Light Flash`)
  (`PaperFlipbookComponent.SetFlipbook` _paperflipbook (`self.FireFlipbook`))
  (`KismetSystemLibrary.Delay` (`PaperFlipbookComponent.GetFlipbookLength` _paperflipbook))
  (`PaperFlipbookComponent.SetFlipbook` (`self.PaperFlipbook`) (`self.IdleFlipbook`)))

(event `Light Flash`
  (bind _pointlight (`self.PointLight`))
  ;[1 1 1] Light flash
  (`SceneComponent.SetHiddenInGame` _pointlight false false)
  (`KismetSystemLibrary.Delay` 0.1)
  (`SceneComponent.SetHiddenInGame` _pointlight true false))

(fn `UserConstructionScript`
  (`parent.UserConstructionScript`))